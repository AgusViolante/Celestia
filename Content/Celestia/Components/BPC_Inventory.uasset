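; BPC_Inventory is an inventory component storing item stacks as an array of item structs, with hotbar removal by index.
; AddItem merges into a stack with room or appends, then notifies the owner through ItemAddedToSlotMessage.
; RemoveItemFromHotbar decrements a stack or blanks the emptied slot.
; FindAnyBlank always reports false and CheckHasSpace never flags stack room, so blanks go unused and full-length inventories report no space.
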(fn AddItem
  (params (ItemInfo :type S%20Item%20Info%20Structure) (ItemQuantity :type Integer))
  (bind _returnvalue (Components|GetOwner))
  (LocalVariables|SetINCItem ItemInfo)
  (LocalVariables|SetINCAmount ItemQuantity)
  (bind (_array_element _array_index) (Utilities|Array|ForEachLoopwithBreak (Variables|Default|GetInventory) :!label _label)
    (:LoopBody
      (if (and (Utilities|Enum|Equal(Enum) (.ItemID (Utilities|Struct|BreakS_ItemInfo _array_element)) (.ItemID (Utilities|Struct|BreakS_ItemInfo (LocalVariables|GetINCItem)))) (<= (+ (.CurrentStack (Utilities|Struct|BreakS_ItemInfo _array_element)) (LocalVariables|GetINCAmount)) (.MaxStack (Utilities|Struct|BreakS_ItemInfo (LocalVariables|GetINCItem)))))
        (LocalVariables|SetFoundItemInfo _array_element)
        (LocalVariables|SetbFoundRoom true)
        (LocalVariables|SetFoundIndex _array_index)
        (goto _label Break)))
    (:Completed
      (if (LocalVariables|GetbFoundRoom)
        (LocalVariables|SetbFoundRoom false)
        (Utilities|Array|SetArrayElem (Variables|Default|GetInventory) (LocalVariables|GetFoundIndex) (Utilities|Struct|MakeS_ItemInfo (.ItemID (Utilities|Struct|BreakS_ItemInfo (LocalVariables|GetINCItem))) (.ItemType (Utilities|Struct|BreakS_ItemInfo (LocalVariables|GetINCItem))) (.ItemName (Utilities|Struct|BreakS_ItemInfo (LocalVariables|GetINCItem))) (.ItemImage (Utilities|Struct|BreakS_ItemInfo (LocalVariables|GetINCItem))) (+ (Utilities|Struct|BreakS_ItemInfo (LocalVariables|GetFoundItemInfo)) (LocalVariables|GetINCAmount)) (.MaxStack (Utilities|Struct|BreakS_ItemInfo (LocalVariables|GetINCItem))) (.Recipe (Utilities|Struct|BreakS_ItemInfo (LocalVariables|GetINCItem))) (.Effectiveness (Utilities|Struct|BreakS_ItemInfo (LocalVariables|GetINCItem))) (.UseAnimation (Utilities|Struct|BreakS_ItemInfo (LocalVariables|GetINCItem))) (.Sell (Utilities|Struct|BreakS_ItemInfo (LocalVariables|GetINCItem))) (.Buy (Utilities|Struct|BreakS_ItemInfo (LocalVariables|GetINCItem))) (.StaminaCost (Utilities|Struct|BreakS_ItemInfo (LocalVariables|GetINCItem))) (.ItemClass (Utilities|Struct|BreakS_ItemInfo (LocalVariables|GetINCItem)))))
        (Class|BPIPlayer|ItemAddedtoSlot(Message) (Components|GetOwner) (Utilities|Struct|MakeS_ItemInfo (.ItemID (Utilities|Struct|BreakS_ItemInfo (LocalVariables|GetINCItem))) (.ItemType (Utilities|Struct|BreakS_ItemInfo (LocalVariables|GetINCItem))) (.ItemName (Utilities|Struct|BreakS_ItemInfo (LocalVariables|GetINCItem))) (.ItemImage (Utilities|Struct|BreakS_ItemInfo (LocalVariables|GetINCItem))) (+ (Utilities|Struct|BreakS_ItemInfo (LocalVariables|GetFoundItemInfo)) (LocalVariables|GetINCAmount)) (.MaxStack (Utilities|Struct|BreakS_ItemInfo (LocalVariables|GetINCItem))) (.Recipe (Utilities|Struct|BreakS_ItemInfo (LocalVariables|GetINCItem))) (.Effectiveness (Utilities|Struct|BreakS_ItemInfo (LocalVariables|GetINCItem))) (.UseAnimation (Utilities|Struct|BreakS_ItemInfo (LocalVariables|GetINCItem))) (.Sell (Utilities|Struct|BreakS_ItemInfo (LocalVariables|GetINCItem))) (.Buy (Utilities|Struct|BreakS_ItemInfo (LocalVariables|GetINCItem))) (.StaminaCost (Utilities|Struct|BreakS_ItemInfo (LocalVariables|GetINCItem))) (.ItemClass (Utilities|Struct|BreakS_ItemInfo (LocalVariables|GetINCItem)))) (LocalVariables|GetFoundIndex))
        (else
          (bind (_bblankfound _index) (CallFunction|FindAnyBlank))
          (if _bblankfound
            (Utilities|Array|SetArrayElem (Variables|Default|GetInventory) _index (Utilities|Struct|MakeS_ItemInfo (.ItemID (Utilities|Struct|BreakS_ItemInfo (LocalVariables|GetINCItem))) (.ItemType (Utilities|Struct|BreakS_ItemInfo (LocalVariables|GetINCItem))) (.ItemName (Utilities|Struct|BreakS_ItemInfo (LocalVariables|GetINCItem))) (.ItemImage (Utilities|Struct|BreakS_ItemInfo (LocalVariables|GetINCItem))) (LocalVariables|GetINCAmount) (.MaxStack (Utilities|Struct|BreakS_ItemInfo (LocalVariables|GetINCItem))) (.Recipe (Utilities|Struct|BreakS_ItemInfo (LocalVariables|GetINCItem))) (.Effectiveness (Utilities|Struct|BreakS_ItemInfo (LocalVariables|GetINCItem))) (.UseAnimation (Utilities|Struct|BreakS_ItemInfo (LocalVariables|GetINCItem))) (.Sell (Utilities|Struct|BreakS_ItemInfo (LocalVariables|GetINCItem))) (.Buy (Utilities|Struct|BreakS_ItemInfo (LocalVariables|GetINCItem))) (.StaminaCost (Utilities|Struct|BreakS_ItemInfo (LocalVariables|GetINCItem))) (.ItemClass (Utilities|Struct|BreakS_ItemInfo (LocalVariables|GetINCItem)))))
            (Class|BPIPlayer|ItemAddedtoSlot(Message) _returnvalue (Utilities|Struct|MakeS_ItemInfo (.ItemID (Utilities|Struct|BreakS_ItemInfo (LocalVariables|GetINCItem))) (.ItemType (Utilities|Struct|BreakS_ItemInfo (LocalVariables|GetINCItem))) (.ItemName (Utilities|Struct|BreakS_ItemInfo (LocalVariables|GetINCItem))) (.ItemImage (Utilities|Struct|BreakS_ItemInfo (LocalVariables|GetINCItem))) (LocalVariables|GetINCAmount) (.MaxStack (Utilities|Struct|BreakS_ItemInfo (LocalVariables|GetINCItem))) (.Recipe (Utilities|Struct|BreakS_ItemInfo (LocalVariables|GetINCItem))) (.Effectiveness (Utilities|Struct|BreakS_ItemInfo (LocalVariables|GetINCItem))) (.UseAnimation (Utilities|Struct|BreakS_ItemInfo (LocalVariables|GetINCItem))) (.Sell (Utilities|Struct|BreakS_ItemInfo (LocalVariables|GetINCItem))) (.Buy (Utilities|Struct|BreakS_ItemInfo (LocalVariables|GetINCItem))) (.StaminaCost (Utilities|Struct|BreakS_ItemInfo (LocalVariables|GetINCItem))) (.ItemClass (Utilities|Struct|BreakS_ItemInfo (LocalVariables|GetINCItem)))) _index)
            (else
              (bind _returnvalue_2 (Utilities|Array|Add (Variables|Default|GetInventory) (Utilities|Struct|MakeS_ItemInfo (.ItemID (Utilities|Struct|BreakS_ItemInfo (LocalVariables|GetINCItem))) (.ItemType (Utilities|Struct|BreakS_ItemInfo (LocalVariables|GetINCItem))) (.ItemName (Utilities|Struct|BreakS_ItemInfo (LocalVariables|GetINCItem))) (.ItemImage (Utilities|Struct|BreakS_ItemInfo (LocalVariables|GetINCItem))) (LocalVariables|GetINCAmount) (.MaxStack (Utilities|Struct|BreakS_ItemInfo (LocalVariables|GetINCItem))) (.Recipe (Utilities|Struct|BreakS_ItemInfo (LocalVariables|GetINCItem))) (.Effectiveness (Utilities|Struct|BreakS_ItemInfo (LocalVariables|GetINCItem))) (.UseAnimation (Utilities|Struct|BreakS_ItemInfo (LocalVariables|GetINCItem))) (.Sell (Utilities|Struct|BreakS_ItemInfo (LocalVariables|GetINCItem))) (.Buy (Utilities|Struct|BreakS_ItemInfo (LocalVariables|GetINCItem))) (.StaminaCost (Utilities|Struct|BreakS_ItemInfo (LocalVariables|GetINCItem))) (.ItemClass (Utilities|Struct|BreakS_ItemInfo (LocalVariables|GetINCItem))))))
              (Class|BPIPlayer|ItemAddedtoSlot(Message) _returnvalue (Utilities|Struct|MakeS_ItemInfo (.ItemID (Utilities|Struct|BreakS_ItemInfo (LocalVariables|GetINCItem))) (.ItemType (Utilities|Struct|BreakS_ItemInfo (LocalVariables|GetINCItem))) (.ItemName (Utilities|Struct|BreakS_ItemInfo (LocalVariables|GetINCItem))) (.ItemImage (Utilities|Struct|BreakS_ItemInfo (LocalVariables|GetINCItem))) (LocalVariables|GetINCAmount) (.MaxStack (Utilities|Struct|BreakS_ItemInfo (LocalVariables|GetINCItem))) (.Recipe (Utilities|Struct|BreakS_ItemInfo (LocalVariables|GetINCItem))) (.Effectiveness (Utilities|Struct|BreakS_ItemInfo (LocalVariables|GetINCItem))) (.UseAnimation (Utilities|Struct|BreakS_ItemInfo (LocalVariables|GetINCItem))) (.Sell (Utilities|Struct|BreakS_ItemInfo (LocalVariables|GetINCItem))) (.Buy (Utilities|Struct|BreakS_ItemInfo (LocalVariables|GetINCItem))) (.StaminaCost (Utilities|Struct|BreakS_ItemInfo (LocalVariables|GetINCItem))) (.ItemClass (Utilities|Struct|BreakS_ItemInfo (LocalVariables|GetINCItem)))) _returnvalue_2))))))))

(fn CheckHasSpace
  (params (ItemInfo :type S%20Item%20Info%20Structure) (ItemQuantity :type Integer))
  (LocalVariables|SetINCItem ItemInfo)
  (LocalVariables|SetINCAmount ItemQuantity)
  (if (>= (Utilities|Array|Length (Variables|Default|GetInventory)) (Variables|Default|GetInventorysyze))
    (bind _array_element (Utilities|Array|ForEachLoopwithBreak (Variables|Default|GetInventory) :!label _label)
      (:LoopBody
        (if (and (Utilities|Enum|Equal(Enum) (.ItemID (Utilities|Struct|BreakS_ItemInfo _array_element)) (.ItemID (Utilities|Struct|BreakS_ItemInfo (LocalVariables|GetINCItem)))) (<= (+ (.CurrentStack (Utilities|Struct|BreakS_ItemInfo _array_element)) (LocalVariables|GetINCAmount)) (.MaxStack (Utilities|Struct|BreakS_ItemInfo (LocalVariables|GetINCItem)))))
          (LocalVariables|SetbFoundSpace false)
          (goto _label Break)))
      (:Completed
        (if (LocalVariables|GetbFoundSpace)
          (LocalVariables|SetbFoundSpace false)
          (return true)
          (else
            (bind _bblankfound (CallFunction|FindAnyBlank))
            (return _bblankfound)))))
    (else
      (return true))))

(fn FindAnyBlank
  (bind (_array_element _array_index) (Utilities|Array|ForEachLoopwithBreak (Variables|Default|GetInventory) :!label _label)
    (:LoopBody
      (if (Utilities|Enum|Equal(Enum) (.ItemID (Utilities|Struct|BreakS_ItemInfo _array_element)) "NewEnumerator0")
        (LocalVariables|SetbFound true)
        (LocalVariables|SetbFoundIndex _array_index)
        (goto _label Break)))
    (:Completed
      (if (LocalVariables|GetbFound)
        (LocalVariables|SetbFound false)
        (return false (LocalVariables|GetbFoundIndex))
        (else
          (return false 0))))))

(fn RemoveItemfromHotbar
  (params (Amount :type Integer) (Index :type Integer))
  (bind _inventory (Variables|Default|GetInventory))
  (bind _output (Utilities|Array|Get(acopy) _inventory Index))
  (bind (_itemid _itemtype _itemname _itemimage _currentstack _maxstack _recipe _effectiveness _useanimation _sell _buy _staminacost _itemclass) (Utilities|Struct|BreakS_ItemInfo _output))
  (bind _returnvalue (- _currentstack Amount))
  (Utilities|Array|SetArrayElem (Variables|Default|GetInventory) Index (select (> _returnvalue 0) (Utilities|Struct|MakeS_ItemInfo _itemid _itemtype _itemname _itemimage _returnvalue _maxstack _recipe _effectiveness _useanimation _sell _buy _staminacost _itemclass) (Utilities|Struct|MakeS_ItemInfo "NewEnumerator0" "NewEnumerator0" "" "/Engine/EngineResources/Black.Black" 0 0 "()" 0 0 0 0 0.0 0))))