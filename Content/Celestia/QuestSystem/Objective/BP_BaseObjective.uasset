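; BP_BaseObjective is the base objective for the Celestia quest system, tracking whether a single objective is active and complete.
; Finishing sets the complete flag, calls CallFinishObjective with itself and prints a debug message.
; It returns its ID when complete, and can finish itself when that ID appears in a supplied completed list.
; Progress is binary, either zero or one.
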(fn ActiveObjective
  (Variables|Default|SetbIsActive true))

(fn FinishObetcive
  (Variables|Default|SetbIsComplete true)
  (Default|CallFinishObjective self)
  (Development|PrintString 0 "Se completo"))

(fn GetrCompletedObjectives
  (if (Variables|Default|GetbIsComplete)
    (return (Utilities|Array|MakeArray (Variables|Default|GetObectiveID)))
    (else
      (return 0))))

(fn SetObjectiveCompletebyID
  (params (CompletedObjectives :type Array%20of%20Strings))
  (if (Utilities|Array|ContainsItem CompletedObjectives (Variables|Default|GetObectiveID))
    (CallFunction|FinishObetcive)))

(fn GetCompletionProgress
  (return (Math|Float|SelectFloat 1.0 0.0 (Variables|Default|GetbIsComplete))))