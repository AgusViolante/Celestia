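; BP_ObjectiveCollection is a composite quest objective that groups sub-objectives and completes once all of them are complete.
; On activation it either starts them one after another when Ordered is set, or all at once.
; Finish events start the next inactive child or recheck completion, while child updates are forwarded as the collection's own.
; Its completion progress is the equal-weight average of the children's progress.
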(event Custom|ForwardUpdateObjective
  (params (Objective :type BP%20Base%20Objective%20Object%20Reference))
  (Default|CallUpdateObjective self))

(event Custom|OnObjectiveFinished
  (params (Objective :type BP%20Base%20Objective%20Object%20Reference))
  (CallFunction|CheckObjectiveFinished)
  (EventDispatchers|UnbindEventfromFinishObjective Objective (delegate Custom|OnObjectiveFinished))
  (Default|CallUpdateObjective self))

(event Custom|OnObjectiveCompleted
  (params (Objective :type BP%20Base%20Objective%20Object%20Reference))
  (EventDispatchers|UnbindEventfromFinishObjective Objective (delegate Custom|OnObjectiveCompleted))
  (CallFunction|ActivateNextObjective (delegate Custom|OnObjectiveCompleted))
  (Default|CallUpdateObjective self))

(event EventActiveObjective
  (|CallParentFunction)
  (for _array_element (Variables|Default|GetSubObjectives)
    (EventDispatchers|BindEventtoUpdateObjective _array_element (delegate Custom|ForwardUpdateObjective)))
  (if (Variables|Default|GetOrdered)
    (CallFunction|ActivateNextObjective (delegate Custom|OnObjectiveCompleted))
    (else
      (for _array_element_2 (Variables|Default|GetSubObjectives)
        (Default|ActiveObjective _array_element_2)
        (EventDispatchers|BindEventtoFinishObjective _array_element_2 (delegate Custom|OnObjectiveFinished)))))
  (Default|CallUpdateObjective self))

(fn CheckObjectiveFinished
  (for _array_element (Variables|Default|GetSubObjectives)
    (if (not (Variables|/Game/Celestia/QuestSystem/Objective/BP_BaseObjective.BP_BaseObjective_C|GetbIsComplete _array_element))
      (return)))
  (CallFunction|FinishObetcive))

(fn ActivateNextObjective
  (params (Event :type Delegate%20%28by%20ref%29))
  (for _array_element (Variables|Default|GetSubObjectives)
    (if (not (Variables|/Game/Celestia/QuestSystem/Objective/BP_BaseObjective.BP_BaseObjective_C|GetbIsActive _array_element))
      (Default|ActiveObjective _array_element)
      (EventDispatchers|BindEventtoFinishObjective _array_element Event)
      (return)))
  (CallFunction|CheckObjectiveFinished))

(fn GetCompletionProgress
  (bind _subobjectives (Variables|Default|GetSubObjectives))
  (for _array_element _subobjectives
    (bind _completionrate (CallFunction|GetCompletionProgress _array_element))
    (LocalVariables|SetCompleteRate (+ (LocalVariables|GetCompleteRate) (/ _completionrate (Math|Conversions|ToFloat(Integer) (Utilities|Array|Length _subobjectives))))))
  (return (LocalVariables|GetCompleteRate)))