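; Quest tracking component that keeps active and finished quests in maps keyed by quest ID.
; Adding a quest skips any already active or finished, then starts it and binds to its updated and completed events.
; Completion moves a quest from the active map to the finished one and refreshes the quest list widget, which is linked to the component through SetWidgetComponent.
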(fn IsQuestActive
  (params (Quest%20To%20Check :type BP%20Quest%20Base%20Object%20Reference))
  (return (Utilities|Map|Contains (Variables|Default|GetActiveQuests) (Variables|/Game/Celestia/QuestSystem/Quests/BP_QuestBase.BP_QuestBase_C|GetQuestID Quest%20To%20Check))))

(fn IsQuestFinished
  (params (Quest%20To%20Check :type BP%20Quest%20Base%20Object%20Reference))
  (return (Utilities|Map|Contains (Variables|Default|GetFinishedQuests) (Variables|/Game/Celestia/QuestSystem/Quests/BP_QuestBase.BP_QuestBase_C|GetQuestID Quest%20To%20Check))))

(fn AddQuest
  (params (Quest%20To%20Add :type BP%20Quest%20Base%20Object%20Reference))
  (if (and (not (CallFunction|IsQuestFinished Quest%20To%20Add)) (not (CallFunction|IsQuestActive Quest%20To%20Add)))
    (Default|StartQuest Quest%20To%20Add)
    (Utilities|Map|Add (Variables|Default|GetActiveQuests) (Variables|/Game/Celestia/QuestSystem/Quests/BP_QuestBase.BP_QuestBase_C|GetQuestID Quest%20To%20Add) Quest%20To%20Add)
    (EventDispatchers|BindEventtoQuestUpdated Quest%20To%20Add (EventDispatchers|CreateEvent :!event UpdateUI))
    (EventDispatchers|BindEventtoCompletedQuest Quest%20To%20Add (EventDispatchers|CreateEvent :!event CompleteQuest))))

(fn CompleteQuest
  (params (CompletedQuest :type BP%20Quest%20Base%20Object%20Reference))
  (bind _questid (Variables|/Game/Celestia/QuestSystem/Quests/BP_QuestBase.BP_QuestBase_C|GetQuestID CompletedQuest))
  (Utilities|Map|Remove (Variables|Default|GetActiveQuests) _questid)
  (Utilities|Map|Add (Variables|Default|GetFinishedQuests) _questid CompletedQuest)
  (Default|UpdateQuestList (Variables|Default|GetQuestUI%20REF)))

(fn UpdateUI
  (Default|UpdateQuestList (Variables|Default|GetQuestUI%20REF)))

(fn SetWidgetComponent
  (params (QuestWidget :type WBP%20Quest%20Window%20Object%20Reference))
  (bind _output_get (Variables|Default|SetQuestUI%20REF QuestWidget))
  (Default|SetsComponent _output_get self)
  (Default|UpdateQuestList _output_get))