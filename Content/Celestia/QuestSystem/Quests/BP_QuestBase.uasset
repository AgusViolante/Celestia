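; BP_QuestBase is the base quest Blueprint, managing a quest's root objective and reporting its progress and completion.
; StartQuest gets the root objective from InitObjectives, a placeholder that only prints a debug string here, then activates it.
; Root completion fires the completed-quest dispatcher, while updates or completion of its direct sub-objectives fire the quest-updated dispatcher, which also fires on start.
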(event Custom|OnQuestCompleted
  (params (Objective :type BP%20Base%20Objective%20Object%20Reference))
  (Default|CallCompletedQuest self))

(event Custom|StartQuest
  (bind _objective (CallFunction|InitObjectives))
  (bind _output_get (Variables|Default|SetObjective%20REF _objective))
  (Default|ActiveObjective _output_get)
  (EventDispatchers|BindEventtoFinishObjective _output_get (delegate Custom|OnQuestCompleted))
  (for _array_element (Variables|/Game/Celestia/QuestSystem/Objective/BP_ObjectiveCollection.BP_ObjectiveCollection_C|GetSubObjectives (Variables|Default|GetObjective%20REF))
    (EventDispatchers|BindEventtoUpdateObjective _array_element (delegate Custom|UpdateQuest))
    (EventDispatchers|BindEventtoFinishObjective _array_element (delegate Custom|UpdateQuest)))
  (Default|CallQuestUpdated))

(event Custom|UpdateQuest
  (params (Objective :type BP%20Base%20Objective%20Object%20Reference))
  (Default|CallQuestUpdated))

(fn ConstructionScript)

(fn InitObjectives
  (Development|PrintString "ParentObjectvie")
  (return 0))