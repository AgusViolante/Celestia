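; BP_NPC is an NPC Blueprint that shows dialogue lines one at a time on screen.
; Each Talk event increments TalkIndex and writes that entry of the Dialogue array into a WBP_Dialogue widget.
; The widget is created for player controller 0 when no valid reference exists, then reused.
; Once the index passes the last line, the widget is removed from its parent, and the index is not reset here.
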(event EventTalk
  (Math|Integer|IncrementInt (Variables|Default|GetTalkIndex)
    (:%20%20
      (if (< (Variables|Default|GetTalkIndex) (Utilities|Array|Length (Variables|Default|GetDialogue)))
        (Variables|Default|GetWBP_DialogueREF
          (:then
            _)
          (:else
            (bind _returnvalue (UserInterface|CreateWidget "/Game/Celestia/NPC/WBP_Dialogue.WBP_Dialogue_C" (Game|GetPlayerController 0)))
            (Variables|Default|SetWBP_DialogueREF _returnvalue)
            (UserInterface|Viewport|AddtoViewport _returnvalue 0)))
        (Rendering|Components|TextRender|SetText (Variables|/Game/Celestia/NPC/WBP_Dialogue.WBP_Dialogue_C|GetDialogueText _returnvalue) (Utilities|Text|ToText(String) (Utilities|Array|Get(acopy) (Variables|Default|GetDialogue) (Variables|Default|GetTalkIndex))))
        (else
          (Widget|RemovefromParent (Variables|Default|GetWBP_DialogueREF)))))))

(fn ConstructionScript)