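; Checkpoint actor that sets the player's respawn point when the player character enters its box trigger.
; On overlap it writes the player's current transform, rather than its own, to SpawnTransform on BP_ThirdPersonGameMode, then swaps the mesh material to show activation.
; The item, inventory-space and gold check functions are stubs that always return false.
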(event OnComponentBeginOverlap(Box)
  (params (OverlappedComponent :type Primitive%20Component%20Object%20Reference) (OtherActor :type Actor%20Object%20Reference) (OtherComp :type Primitive%20Component%20Object%20Reference) (OtherBodyIndex :type Integer) (bFromSweep :type Boolean) (SweepResult :type Hit%20Result%20Structure%20%28by%20ref%29))
  (bind _returnvalue (Game|GetPlayerCharacter 0))
  (if (== OtherActor _returnvalue)
    (bind _asbp_third_person_game_mode (Utilities|Casting|CastToBP_ThirdPersonGameMode (Game|GetGameMode)))
    (Variables|/Game/Celestia/Blueprints/BP_ThirdPersonGameMode.BP_ThirdPersonGameMode_C|SetSpawn%20Transform _asbp_third_person_game_mode (Transformation|GetActorTransform _returnvalue))
    (CallFunction|ChangeColor)))

(event Custom|ChangeColor
  (Rendering|Material|SetMaterial (Variables|Default|GetStaticMesh) 0 "/Engine/MapTemplates/Materials/BasicAsset01.BasicAsset01"))

(event EventBeginPlay)

(event Collision|EventActorBeginOverlap
  (params (OtherActor :type Actor%20Object%20Reference)))

(event EventTick
  (params (DeltaSeconds :type Float%20%28single-precision%29)))

(fn ConstructionScript)

(fn CheckHasItem
  (params (KeyName :type String))
  (return false))

(fn CheckInventorySpace
  (params (item%20info :type S%20Item%20Info%20Structure) (item%20amount :type Integer))
  (return false))

(fn CheckPlayerGold
  (params (AmountRequired :type Integer))
  (return false))