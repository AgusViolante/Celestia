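; BP_BaseItem is a base actor for world items that a CelestiaCharacter picks up by interacting.
; The construction script fills ItemInfo from the DT_ItemData row named after its ItemID enum.
; Interact checks inventory space through a message call, then adds one item and destroys the actor.
; A DoOnce with no reset gates Interact, so a failed space check also blocks later attempts.
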(event EventInteract
  (params (Interactor :type Actor%20Object%20Reference))
  (Utilities|FlowControl|DoOnce false
    (:Completed
      (bind _ascelestia_character (Utilities|Casting|CastToCelestiaCharacter Interactor))
      (bind _hasspace (Class|BPIPlayer|CheckInventorySpace(Message) _ascelestia_character (Variables|Default|GetItemInfo) 1))
      (if _hasspace
        (Class|BPIPlayer|AddItem(Message) Interactor (Variables|Default|GetItemInfo) 1)
        (Actor|DestroyActor)))))

(fn ConstructionScript
  (bind _returnvalue (Utilities|GetDataTableRow "/Game/Celestia/Structure/DT_ItemData.DT_ItemData" (Utilities|String|StringToName (Utilities|String|EnumtoString (.ItemID (Utilities|Struct|BreakS_ItemInfo (Variables|Default|GetItemInfo))))))
    (:then
      (Variables|Default|SetItemInfo _returnvalue))))