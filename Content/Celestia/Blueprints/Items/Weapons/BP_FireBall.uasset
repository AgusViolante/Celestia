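; BP_FireBall is a fireball weapon actor that deals magic damage on overlap with any actor other than its instigator.
; Targets with a HealthComponent take damage built from the instigator's StatsComponent MagicAttack, with a MagicCrit percentage roll boosting part of it and setting the critical flag.
; Any non-instigator overlap spawns a Niagara effect slightly above the fireball and destroys it.
; It also prints the damaged target's name.
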(event Collision|EventActorBeginOverlap
  (params (OtherActor :type Actor%20Object%20Reference))
  (bind _returnvalue (Game|GetInstigator))
  (bind _returnvalue_2 (Math|Random|RandomFloatinRange 0.0 1e+02))
  (bind _returnvalue_3 (Actor|GetComponentbyClass OtherActor "/Script/Celestia.HealthComponent"))
  (bind _returnvalue_4 (Actor|GetComponentbyClass _returnvalue "/Script/Celestia.StatsComponent"))
  (bind _returnvalue_5 (Class|StatsComponent|GetStatValue _returnvalue_4 "MagicAttack"))
  (bind _returnvalue_6 (Class|StatsComponent|GetStatValue _returnvalue_4 "MagicCrit"))
  (bind _returnvalue_7 (<= _returnvalue_2 _returnvalue_6))
  (if (!= OtherActor _returnvalue)
    (Utilities|IsValid _returnvalue_3
      (:Is%20Valid
        (Development|PrintString (Utilities|GetDisplayName OtherActor))
        (Class|HealthComponent|TakeDamage _returnvalue_3 (+ (Math|Float|SelectFloat (* _returnvalue_5 1.5) _returnvalue_5 _returnvalue_7) _returnvalue_5 0.0) _returnvalue_7))
      (:Is%20Not%20Valid
        _))
    (Niagara|SpawnSystematLocation "/Game/ArrowTrail/FX/NS_ArrowTrail_Basic_02.NS_ArrowTrail_Basic_02" (+ (Transformation|GetActorLocation) "0.000000,0.000000,50.000000"))
    (Actor|DestroyActor)))

(fn ConstructionScript)