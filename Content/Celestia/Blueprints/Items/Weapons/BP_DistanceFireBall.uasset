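; BP_DistanceFireBall is a fireball attack that damages enemies overlapping its sphere shortly after spawning.
; After a brief delay, it applies damage to each EnemyBase with a HealthComponent, scaled from the instigator's MagicAttack stat with a MagicCrit-based critical roll.
; Each hit spawns a Niagara magic-area effect at the actor's location and leads into a delayed self-destroy, which only runs when something is hit.
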(event EventBeginPlay
  (bind _returnvalue (Game|GetInstigator))
  (bind _returnvalue_2 (Math|Random|RandomFloatinRange 0.0 1e+02))
  (bind _returnvalue_3 (Actor|GetComponentbyClass _returnvalue "/Script/Celestia.StatsComponent"))
  (bind _returnvalue_4 (Class|StatsComponent|GetStatValue _returnvalue_3 "MagicAttack"))
  (bind _returnvalue_5 (Class|StatsComponent|GetStatValue _returnvalue_3 "MagicCrit"))
  (bind _returnvalue_6 (<= _returnvalue_2 _returnvalue_5))
  (Utilities|FlowControl|Delay 0.1)
  (for _array_element (Collision|GetOverlappingActors (Variables|Default|GetSphere) "/Script/Celestia.EnemyBase" :!class /Script/Engine.PrimitiveComponent)
    (Utilities|IsValid (Actor|GetComponentbyClass _array_element "/Script/Celestia.HealthComponent")
      (:Is%20Valid
        (Class|HealthComponent|TakeDamage (Actor|GetComponentbyClass _array_element "/Script/Celestia.HealthComponent") (+ (Math|Float|SelectFloat (* _returnvalue_4 1.5) _returnvalue_4 _returnvalue_6) _returnvalue_4 0.0) _returnvalue_6 false)
        (Niagara|SpawnSystematLocation "/Game/Free_Magic/VFX_Niagara/NS_Free_Magic_Area2.NS_Free_Magic_Area2" (Transformation|GetActorLocation))
        (Utilities|FlowControl|Delay 2.0)
        (Actor|DestroyActor)))))

(fn ConstructionScript)