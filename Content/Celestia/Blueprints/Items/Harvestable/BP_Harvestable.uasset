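; BP_Harvestable is a harvestable world object that takes damage and grants items to the player when destroyed.
; BeginPlay picks the reward item from the required tool type and rolls a random amount.
; When damage depletes its health, it looks up the reward in DT_ItemData, sends it to player 0's character and destroys itself.
; The construction script applies the configured mesh, and CheckRequirements reports whether a given tool matches.
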(event Game|Damage|EventAnyDamage
  (params (Damage :type Float%20%28single-precision%29) (DamageType :type Damage%20Type%20Object%20Reference) (InstigatedBy :type Controller%20Object%20Reference) (DamageCauser :type Actor%20Object%20Reference))
  (bind _output_get (Variables|Default|SetHarvestableHealth (Math|Float|Truncate (- (Variables|Default|GetHarvestableHealth) Damage))))
  (if (<= _output_get 0)
    (bind _returnvalue (Utilities|GetDataTableRow "/Game/Celestia/Structure/DT_ItemData.DT_ItemData" (Utilities|String|StringToName (Utilities|String|EnumtoString (Variables|Default|GetRewardID))))
      (:then
        (Class|BPIPlayer|AddItem(Message) (Game|GetPlayerCharacter 0) _returnvalue (Variables|Default|GetRewardAmount))
        (Actor|DestroyActor)))))

(event EventBeginPlay
  (Variables|Default|SetRewardID (Utilities|Select :Index (Variables|Default|GetToolRequirement) :NewEnumerator0 "NewEnumerator9" :NewEnumerator1 "NewEnumerator10"))
  (Variables|Default|SetRewardAmount (Math|Random|RandomIntegerinRange 3 5)))

(fn ConstructionScript
  (Components|StaticMesh|SetStaticMesh (Variables|Default|GetStaticMesh) (Variables|Default|GetHarvestMesh)))

(fn CheckRequirements
  (params (ToolUsed :type E_ToolID%20Enum :default "NewEnumerator0"))
  (return (Utilities|Enum|Equal(Enum) ToolUsed (Variables|Default|GetToolRequirement))))