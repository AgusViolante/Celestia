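; BP_InteractableItem is a pickup item actor that hands its item data to the player when interacted with.
; The construction script uses the chosen item name enum as a row key in DT_Items, setting the mesh and storing the row as ItemInfo.
; BeginPlay caches the player as BP_Player, and Interact passes ItemInfo to its PickUpItem before destroying the actor.
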(event EventBeginPlay
  (bind _asbp_player (Utilities|Casting|CastToBP_Player (Game|GetPlayerCharacter 0)))
  (Variables|Default|SetAs%20BP%20Player%20REF _asbp_player))

(event EventInteract
  (Default|PickUpItem (Variables|Default|GetAs%20BP%20Player%20REF) (Variables|Default|GetItemInfo))
  (Actor|DestroyActor))

(fn ConstructionScript
  (bind _returnvalue (Utilities|GetDataTableRow "/Game/Celestia/Structure/DT_Items.DT_Items" (Utilities|String|StringToName (Utilities|String|EnumtoString (Variables|Default|GetItemNames))))
    (:then
      (Components|StaticMesh|SetStaticMesh (Variables|Default|GetAdaptableItemMesh) (.StaticMesh (Utilities|Struct|BreakS_ItemInfo _returnvalue)))
      (Variables|Default|SetItemInfo _returnvalue))))