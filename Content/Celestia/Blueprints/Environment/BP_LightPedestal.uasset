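; BP_LightPedestal is a pedestal that takes a dungeon light crystal from the player's inventory.
; TryConsumeCrystalFromInventory scans BPC_Inventory for an item class derived from BP_LightCrystalDungeon1, removes the first match and returns whether it succeeded.
; On success it updates the player's hotbar UI and advances the hard-coded "Pedestal_1" Location quest objective, both through player message calls.
; The event graph and construction script are empty.
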(event EventBeginPlay)

(event Collision|EventActorBeginOverlap
  (params (OtherActor :type Actor%20Object%20Reference)))

(event EventTick
  (params (DeltaSeconds :type Float%20%28single-precision%29)))

(fn ConstructionScript)

(fn TryConsumeCrystalfromInventory
  (params (PlayerActor :type Actor%20Object%20Reference))
  (bind _returnvalue (Actor|GetComponentbyClass PlayerActor "/Game/Celestia/Components/BPC_Inventory.BPC_Inventory_C"))
  (Utilities|IsValid _returnvalue
    (:Is%20Valid
      (for (_array_element _array_index) (Variables|/Game/Celestia/Components/BPC_Inventory.BPC_Inventory_C|GetInventory _returnvalue)
        (if (Utilities|ClassIsChildOf (.ItemClass (Utilities|Struct|BreakS_ItemInfo _array_element)) "/Game/Celestia/Blueprints/Items/Props/BP_LightCrystalDungeon1.BP_LightCrystalDungeon1_C")
          (Default|RemoveItem _returnvalue _array_element)
          (Class|BPIPlayer|UpdateHotbarUI(Message) PlayerActor _array_index)
          (bind _questcompnent (Class|BPIQuestUtilities|GetQuestComponent(Message) PlayerActor))
          (Class|QuestComponent|UpdateObjective _questcompnent "Location" "Pedestal_1")
          (return true)))
      (return false))
    (:Is%20Not%20Valid
      (return false))))